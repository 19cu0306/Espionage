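; Security guard character Blueprint that speeds up while it sees the player and ends the game on a catch.
; Each Tick it reads the catch and sighting state from its AI_SecurityCharacter controller.
; A catch opens the GameOver level; otherwise, a sighting raises movement speed by a fixed, frame-rate-dependent step up to the run maximum.
; Without a sighting, speed snaps back to walking.
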(event `self.ReceiveTick`
  (params (DeltaSeconds :type "Float (single-precision)"))
  (bind _charactermovement (`self.CharacterMovement`))
  (bind _walkspeed (`self.WalkSpeed`))
  (bind _asai_security_character (cast `AI_SecurityCharacter` (`AIBlueprintHelperLibrary.GetAIController` self)))
  (if (`AI_SecurityCharacter.isCatchActor` _asai_security_character)
    (`GameplayStatics.OpenLevel` "GameOver")
    (elif (`AI_SecurityCharacter.GetIsSawPlayer` _asai_security_character)
      (bind _output_get (set `self.CurrentRunSpeed` (`KismetMathLibrary.FClamp` (+ (`self.CurrentRunSpeed`) 25.0) (`self.WalkSpeed`) (`self.maxRunSpeed`))))
      (set `CharacterMovementComponent.MaxWalkSpeed` _output_get _charactermovement)
      (else
        (set `CharacterMovementComponent.MaxWalkSpeed` _walkspeed _charactermovement)
        (set `self.CurrentRunSpeed` _walkspeed)))))

(fn `UserConstructionScript`)
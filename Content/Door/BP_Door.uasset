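; Key-locked door for the espionage character that swings open on yaw through a timeline when a player holding the DoorKey enters its trigger.
; Opening also shows the Kari widget and clears the key objective widget; leaving the trigger with the key reverses the timeline.
; Without the key, it shows the Kagi widget for three seconds, then displays and stores a find-door-key objective widget.
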(event `self.Trigger.OnComponentBeginOverlap`
  (params (OverlappedComponent :type "PrimitiveComponent Object Reference") (OtherActor :type "Actor Object Reference") (OtherComp :type "PrimitiveComponent Object Reference") (OtherBodyIndex :type Integer) (bFromSweep :type Boolean) (SweepResult :type "HitResult Structure (by ref)"))
  (bind _asespionage_character_bp (cast `/Game/ThirdPersonBP/Blueprints/EspionageCharacterBP` OtherActor))
  (if (`/Game/ThirdPersonBP/Blueprints/EspionageCharacterBP.Door_Key` _asespionage_character_bp)
    (bind _returnvalue (`|CreateWidget` "/Game/0301tuika/kari.kari_C"))
    (`UserWidget.AddToViewport` _returnvalue 0)
    (`Widget.RemoveFromParent` (`self.Target_DoorKey`))
    (bind (_direction _rotation) (`Timeline|TimeLine` :!label _label)
      (:`Update`
        (`self.K2_SetActorRotation` (`KismetMathLibrary.MakeRotator` 0.0 0.0 _rotation))))
    (else
      (bind _returnvalue_2 (`|CreateWidget` "/Game/0204_tuika/teroppu/misiyou/kagi.kagi_C"))
      (`UserWidget.AddToViewport` _returnvalue_2 0)
      (`KismetSystemLibrary.Delay` 3.0)
      (`Widget.RemoveFromParent` _returnvalue_2)
      (bind _returnvalue_3 (`|CreateWidget` "/Game/0218tuika/Target_Find_DoorKey_BP.Target_Find_DoorKey_BP_C"))
      (bind _output_get (set `self.Target_DoorKey` _returnvalue_3))
      (`UserWidget.AddToViewport` _returnvalue_3 0)
      (`UserWidget.AddToViewport` _output_get 0))))

(event `self.Trigger.OnComponentEndOverlap`
  (params (OverlappedComponent :type "PrimitiveComponent Object Reference") (OtherActor :type "Actor Object Reference") (OtherComp :type "PrimitiveComponent Object Reference") (OtherBodyIndex :type Integer))
  (bind _asespionage_character_bp (cast `/Game/ThirdPersonBP/Blueprints/EspionageCharacterBP` OtherActor))
  (if (`/Game/ThirdPersonBP/Blueprints/EspionageCharacterBP.Door_Key` _asespionage_character_bp)
    (goto _label :!via `Reverse`)))

(fn `UserConstructionScript`)